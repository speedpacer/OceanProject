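; BP_Buoy is an ocean buoy actor with a BuoyancyMovement component and a debug view of that component's test points.
; When DebugMode is on, it draws a red sphere per test point, sized by its volume radius.
; The construction script draws long-lived spheres, while BeginPlay and Tick share a short-lived draw that refreshes each frame.
; Sphere centers add point offsets to world location without applying rotation.
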(event `self.ReceiveBeginPlay`
  (if (and (`self.DebugMode`) (> (`KismetArrayLibrary.Array_Length` (`BuoyancyMovementComponent.TestPoints` (`self.BuoyancyMovement`))) 0)) :!label _label
    (for _array_element (`BuoyancyMovementComponent.TestPoints` (`self.BuoyancyMovement`))
      (bind (_location _buoyancy _volumeradius) (break `BuoyancyMovementComponent.BuoyancyTestPoint` _array_element))
      (`KismetSystemLibrary.DrawDebugSphere` (+ (`SceneComponent.K2_GetComponentLocation`) _location) _volumeradius 12 (struct :`R` 1.0 :`A` 1.0) 0.05))))

(event `self.ReceiveTick`
  (params (DeltaSeconds :type "Float (single-precision)"))
  (goto _label))

(event `self.ReceiveActorBeginOverlap`
  (params (OtherActor :type "Actor Object Reference")))

(fn `UserConstructionScript`
  (if (and (`self.DebugMode`) (> (`KismetArrayLibrary.Array_Length` (`BuoyancyMovementComponent.TestPoints` (`self.BuoyancyMovement`))) 0))
    (for _array_element (`BuoyancyMovementComponent.TestPoints` (`self.BuoyancyMovement`))
      (bind (_location _buoyancy _volumeradius) (break `BuoyancyMovementComponent.BuoyancyTestPoint` _array_element))
      (`KismetSystemLibrary.DrawDebugSphere` (+ (`SceneComponent.K2_GetComponentLocation`) _location) _volumeradius 12 (struct :`R` 1.0 :`A` 1.0) 10.0))))